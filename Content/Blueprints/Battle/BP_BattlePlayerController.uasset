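; Player controller for turn-based battles, owning the battle UI and the player's side of each turn.
; On begin play it creates the battle widget, shows the cursor and, after a short delay, hands the character sub-widget to the active character.
; StartTurn plays the player-turn animation before revealing the character's widget.
; Attack (currently adding zero HP) and LaunchSkill both end by hiding that widget and starting the game mode's enemy turn.
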(event `self.ReceiveBeginPlay`
  (`self.UI_Management`)
  (set `self.bShowMouseCursor` true)
  (`KismetSystemLibrary.Delay` 0.2)
  (set `/Game/Blueprints/Battle/BP_BattleCharacter.Character Battle UI` (`/Game/UI/Battle/WBP_BattleUI.BP_CharacterBattleUI` (`self.BattleUI`)) (`self.ActualChara`)))

(event `StartTurn`
  (bind _battleui (`self.BattleUI`))
  (bind _playerturn (`/Game/UI/Battle/WBP_BattleUI.PlayerTurn` _battleui))
  (`UserWidget.PlayAnimation` _battleui _playerturn 0.0 1 "Forward" 1.0 false)
  (`KismetSystemLibrary.Delay` (`WidgetAnimation.GetEndTime` _playerturn))
  (`SceneComponent.SetVisibility` (`/Game/Blueprints/Battle/BP_BattleCharacter_Player.Widget` (`self.ActualChara`)) true false))

(fn `Attack`
  (bind _outitem (`/Game/Blueprints/Battle/BP_BattleGameMode.SelectEnnemy` (`/Game/Blueprints/Battle/BP_FL_Getters.GetBattleGameMode`)))
  (`/Game/Blueprints/Battle/BP_BattleCharacter.AddHP` _outitem 0.0)
  (`self.EndTurn`))

(fn `EndTurn`
  (`SceneComponent.SetVisibility` (`/Game/Blueprints/Battle/BP_BattleCharacter_Player.Widget` (`self.ActualChara`)) false false)
  (`/Game/Blueprints/Battle/BP_BattleGameMode.EnemiesTurn` (`/Game/Blueprints/Battle/BP_FL_Getters.GetBattleGameMode`)))

(fn `LaunchSkill`
  (params (Skill :type "/Game/Blueprints/Data/BP_Skills Object Reference"))
  (`/Game/Blueprints/Data/BP_Skills.LaunchAction` Skill (`/Game/Blueprints/Battle/BP_FL_Getters.GetBattleGameMode`))
  (`self.EndTurn`))

(fn `UI_Management`
  (bind _returnvalue (`|CreateWidget` "/Game/UI/Battle/WBP_BattleUI.WBP_BattleUI_C"))
  (bind _output_get (set `self.BattleUI` _returnvalue))
  (`UserWidget.AddToViewport` _output_get 0))

(fn `UserConstructionScript`)