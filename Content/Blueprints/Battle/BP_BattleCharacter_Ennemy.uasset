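; Enemy character for the battle mode, configured from EnemyData and registered in the game mode's enemy list on BeginPlay.
; Initialisation sets the name on its battle UI widget, tints the mesh through a dynamic material and fills HP to max.
; Attack passes the data's attack value to the active character's AddHP, plays an animation and returns its length.
; Tick prints HP for debugging, and OnFire only decrements a 3Ticks counter.
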(event `self.ReceiveBeginPlay`
  (bind _aswbp_character_battle_ui (cast `/Game/UI/Battle/WBP_CharacterBattleUI` (`WidgetComponent.GetWidget` (`self.Widget`))))
  (set `self.Character Battle UI` _aswbp_character_battle_ui)
  (`KismetArrayLibrary.Array_Add` (`/Game/Blueprints/Battle/BP_BattleGameMode.Ennemies` (`/Game/Blueprints/Battle/BP_FL_Getters.GetBattleGameMode`)) self)
  (`self.Initialisation`))

(event `self.ReceiveTick`
  (params (DeltaSeconds :type "Float (single-precision)"))
  (`KismetSystemLibrary.PrintString` (`KismetStringLibrary.Conv_DoubleToString` (`self.HP`)) true true (struct :`G` 0.66 :`B` 1.0 :`A` 1.0) 0.0))

(fn `Attack`
  (returns (animationLenght :type "Float (single-precision)"))
  (locals (Animaiton :type "AnimationAsset Object Reference" :default "/Script/Engine.AnimSequence'/Game/Characters/Mannequins/Anims/Pistol/MM_Pistol_DryFire.MM_Pistol_DryFire'"))
  (`self.AddHP` (`/Game/Blueprints/Battle/BP_BattlePlayerController.ActualChara` (`/Game/Blueprints/Battle/BP_FL_Getters.GetBattleController`)) (`KismetMathLibrary.Conv_IntToDouble` (`/Game/Blueprints/Data/BP_Ennemy.Attack` (`self.EnemyData`))))
  (`SkeletalMeshComponent.PlayAnimation` (`self.Mesh`) (`local.Animaiton`) false)
  (return (`AnimationAsset.GetPlayLength` (`local.Animaiton`))))

(fn `Initialisation`
  (`/Game/UI/Battle/WBP_CharacterBattleUI.UpdateName` (`self.Character Battle UI`) (`KismetTextLibrary.Conv_StringToText` (`/Game/Blueprints/Data/BP_Ennemy.Name` (`self.EnemyData`))))
  (bind _returnvalue (`KismetMaterialLibrary.CreateDynamicMaterialInstance` "/Game/Material/M_EnnemyMat.M_EnnemyMat"))
  (bind _output_get (set `self.Material` _returnvalue))
  (`PrimitiveComponent.SetMaterial` (`self.Mesh`) 0 _output_get)
  (`MaterialInstanceDynamic.SetVectorParameterValue` (`self.Material`) "Color" (`/Game/Blueprints/Data/BP_Ennemy.Color` (`self.EnemyData`)))
  (bind _output_get_2 (set `self.HPMax` (`KismetMathLibrary.Conv_IntToDouble` (`/Game/Blueprints/Data/BP_Ennemy.HPMax` (`self.EnemyData`)))))
  (`self.ChangeHP` _output_get_2))

(fn `OnFire`
  (for _ (`|MakeArray` (`self.3Ticks`))
    (set `self.3Ticks` (- (`self.3Ticks`) 1))))

(fn `UserConstructionScript`
  (`parent.UserConstructionScript`))